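; Test actor that shows TouchEngine (TouchDesigner) output on a plane and adds a node render widget to the viewport on BeginPlay.
; The construction script creates a dynamic instance of the ToeOut_stereo material on the plane.
; At each TouchEngine frame end, it feeds the left display wall output texture into that material, printing errors on failure.
; A right-channel texture branch exists but is disconnected and never runs.
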(event `self.TouchEngineComponent.OnEndFrame`
  (params (IsSuccessful :type Boolean) (Result :type "ECookFrameResult Enum" :default "Success") (FrameData :type "TouchEngineOutputFrameData Structure (by ref)"))
  (bind _mid (`self.MID`))
  (`|ExecutionSequence`
    (:`then_0`
      (bind (_value _result) (`|TouchOutputK2Node` (`self.TouchEngineComponent`) "moxg_out_Display_Wall_l"))
      (if _result
        (`/Engine/EditorBlueprintResources/StandardMacros.IsValid` _mid
          (:`Is Valid`
            (`MaterialInstanceDynamic.SetTextureParameterValue` _mid "TETexIn" _value))
          (:`Is Not Valid`
            (`KismetSystemLibrary.PrintString` "invalid material" true true (struct :`R` 1.0 :`B` 0.233351 :`A` 1.0))))
        (else
          (`KismetSystemLibrary.PrintString` "error getting output L" true true (struct :`R` 1.0 :`G` 0.119154 :`A` 1.0)))))))

(event `self.ReceiveBeginPlay`
  (bind _returnvalue (`|CreateWidget` "/Game/BP_NodeRenderWidget.BP_NodeRenderWidget_C" (`GameplayStatics.GetPlayerController` 0)))
  (bind _output_get (set `self.RenderWidget` _returnvalue))
  (`UserWidget.AddToViewport` _output_get 0))

(fn `UserConstructionScript`
  (bind _returnvalue (`PrimitiveComponent.CreateDynamicMaterialInstance` (`self.Plane`) 0 "/Game/td/toeOut_stereo.toeOut_stereo" "None"))
  (set `self.MID` _returnvalue))