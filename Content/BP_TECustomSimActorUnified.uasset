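; nDisplay simulation actor that runs a TouchDesigner TOX, optionally chosen by command line, through TouchEngine.
; Each frame it feeds stereo textures into screen materials and dispatches Ableton and Lisa JSON audio commands.
; Primary or standalone nodes send input and Pharus tracking to TouchDesigner.
; They also rebroadcast its encoded BSON output as binary cluster events that nodes feed back into the TOX; simOnly bypasses the broadcast.
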(event `self.TouchEngineComponent.OnEndFrame`
  (params (IsSuccessful :type Boolean) (Result :type "ECookFrameResult Enum" :default "Success") (FrameData :type "TouchEngineOutputFrameData Structure (by ref)"))
  (bind _datbsonin (`self.DatBsonIn`))
  (bind _touchenginecomponent (`self.TouchEngineComponent`))
  (bind _processclusterdata (`self.ProcessClusterData`))
  (if (`self.ToxLoaded`)
    (`|ExecutionSequence`
      (:`then_0`
        (if true
          (bind _returnvalue (`self.GetScreenProcMeshes`))
          (for (_ _array_index) _returnvalue
            ;[0.15 0.08118 0.03921 0.5] grab frame from TD
            (`|ExecutionSequence`
              (:`then_2`
                (bind _returnvalue_2 (`KismetStringLibrary.Concat_StrStr` "moxg_out_" (`|GetArrayItem` (`self.aScreenNames`) _array_index)))
                (bind (_value _result) (`|TouchOutputK2Node` _touchenginecomponent (`KismetStringLibrary.Concat_StrStr` _returnvalue_2 "_l")))
                (if _result
                  (bind _output (`|GetArrayItem` (`self.aMIDs`) _array_index))
                  (`/Engine/EditorBlueprintResources/StandardMacros.IsValid` _output
                    (:`Is Valid`
                      (`MaterialInstanceDynamic.SetTextureParameterValue` _output "TETexInR" _value))
                    (:`Is Not Valid`
                      (`KismetSystemLibrary.PrintString` "invalid material" true true (struct :`R` 1.0 :`B` 0.233351 :`A` 1.0) :!label _label)))
                  (else
                    (`KismetSystemLibrary.PrintString` "error getting output L" true true (struct :`R` 1.0 :`G` 0.119154 :`A` 1.0)))))
              (:`then_3`
                (bind (_value_2 _result_2) (`|TouchOutputK2Node` _touchenginecomponent (`KismetStringLibrary.Concat_StrStr` _returnvalue_2 "_r")))
                (if _result_2
                  (`/Engine/EditorBlueprintResources/StandardMacros.IsValid` _output
                    (:`Is Valid`
                      (`MaterialInstanceDynamic.SetTextureParameterValue` _output "TETexIn" _value_2))
                    (:`Is Not Valid`
                      (goto _label)))
                  (else
                    (`KismetSystemLibrary.PrintString` "error getting output R" true true (struct :`R` 1.0 :`G` 0.119154 :`A` 1.0)))))))))
      (:`then_1`
        (`|ExecutionSequence`
          (:`then_0`
            ;[0.15 0.0995 0.03464 0.5] TD to DAT
            (bind (_value_3 _result_3 _framelastupdated) (`|TouchOutputK2Node` (`self.TouchEngineComponent`) "moxf_out_encoded_bson"))
            (`|ExecutionSequence`
              (:`then_0`
                (if _result_3
                  (bind _output_get (set `self.DatBsonIn` _value_3))
                  (`|ExecutionSequence`
                    (:`then_0`
                      (for _index (range (`TouchEngineDAT.numRows` _output_get))
                        (for _index_2 (range (`TouchEngineDAT.numColumns` _output_get))
                          (bind _returnvalue_3 (`TouchEngineDAT.GetCell` _output_get _index_2 _index))
                          (`KismetSystemLibrary.PrintString` (`KismetStringLibrary.Concat_StrStr` "FROM TD:" (`self.CellText`) _returnvalue_3) true true (struct :`R` 1.0 :`G` 0.27474 :`B` 0.618986 :`A` 1.0) 2.0 "bsoncell"))))
                    (:`then_1`
                      ; send to cluster nodes >>
                      (switch `EDisplayClusterNodeRole` (`DisplayClusterBlueprintLib.GetClusterRole`)
                        (:`None`
                          _)
                        (:`Primary`
                          _))
                      (`/Engine/EditorBlueprintResources/StandardMacros.IsValid` _datbsonin
                        (:`Is Valid`
                          (bind _returnvalue_4 (`TouchEngineDAT.GetCell` _datbsonin 0 0))
                          (bind _returnvalue_5 (`MoxTdUtilBPLibrary.StringToBytes` _returnvalue_4))
                          ;; cluster event / bypass switch
                          (if _processclusterdata
                            (`DisplayClusterBlueprintLib.EmitClusterEventBinary` (make `DisplayClusterClusterEventBinary` 1 _returnvalue_5))
                            (`KismetSystemLibrary.PrintString` (`KismetStringLibrary.Concat_StrStr` "EMITTING BINARY " _returnvalue_4) true true (struct :`G` 1.0 :`B` 0.229809 :`A` 1.0) 2.0 "pri_emit")
                            (else
                              ; >> cluster node in
                              (bind _returnvalue_6 (`MoxTdUtilBPLibrary.BytesToString` (select `bool` _processclusterdata :`false` _returnvalue_5 :`true` (`.EventData` (break `DisplayClusterClusterEventBinary` (stale `self.OnClusterEventBinary` Event)))) :!label _label_2))
                              (`|ExecutionSequence`
                                (:`then_0`
                                  (bind _result_4 (`|TouchInputK2Node` (`self.TouchEngineComponent`) "moxf_in_encoded_bson" (`|MakeArray` _returnvalue_6)))
                                  (`KismetSystemLibrary.PrintString` (`KismetStringLibrary.Concat_StrStr` "BSON NODE SET RESULT: " (`KismetStringLibrary.Conv_BoolToString` _result_4))))
                                (:`then_1`
                                  (`KismetSystemLibrary.PrintString` (`KismetStringLibrary.Concat_StrStr` "cluster IN: " _returnvalue_6) true true (struct :`G` 0.66 :`B` 1.0 :`A` 1.0) 2.0 "cluster in")))))))))
                  (else
                    (`KismetSystemLibrary.PrintString` "FAIL get DAT" true true (struct :`R` 0.557292 :`B` 0.056032 :`A` 1.0) 1.0))))
              (:`then_1`
                (`KismetSystemLibrary.PrintString` (`KismetStringLibrary.Conv_Int64ToString` _framelastupdated) true true (struct :`R` 0.143515 :`G` 0.013095 :`B` 1.0 :`A` 1.0) 2.0 "td_dat_frame"))))
          (:`then_1`
            ; error output from TD
            (bind (_value_4 _result_5 _framelastupdated_2) (`|TouchOutputK2Node` (`self.TouchEngineComponent`) "moxf_out_err"))
            (`|ExecutionSequence`
              (:`then_0`
                (if _result_5
                  (bind _output_get_2 (set `self.DatErrIn` _value_4))
                  (`|ExecutionSequence`
                    (:`then_0`
                      (for _index_3 (range (`TouchEngineDAT.numRows` _output_get_2))
                        (for _index_4 (range (`TouchEngineDAT.numColumns` _output_get_2))
                          (bind _returnvalue_7 (`TouchEngineDAT.GetCell` _output_get_2 _index_4 _index_3))
                          (`KismetSystemLibrary.PrintString` (`KismetStringLibrary.Concat_StrStr` "ERR: " _returnvalue_7) true true (struct :`R` 1.0 :`G` 0.27474 :`B` 0.618986 :`A` 1.0) 2.0 "ERR DAT")))))
                  (else
                    (`KismetSystemLibrary.PrintString` "FAIL get DAT" true true (struct :`R` 0.557292 :`B` 0.056032 :`A` 1.0) 1.0))))
              (:`then_1`
                (`KismetSystemLibrary.PrintString` (`KismetStringLibrary.Conv_Int64ToString` _framelastupdated_2) true true (struct :`R` 0.143515 :`G` 0.013095 :`B` 1.0 :`A` 1.0) 2.0 "td_dat_frame"))))))
      (:`then_2`
        ; Audio Interface
        (`|ExecutionSequence`
          (:`then_0`
            (bind (_value_5 _result_6) (`|TouchOutputK2Node` (`self.TouchEngineComponent`) "moxf_out_ableton"))
            (if _result_6
              (bind _output_get_3 (set `self.DatAbletonIn` _value_5))
              (for _index_5 (range (- (`TouchEngineDAT.numRows` _output_get_3) 1) 1)
                (for _index_6 (range (`TouchEngineDAT.numColumns` _output_get_3))
                  (bind _returnvalue_8 (`TouchEngineDAT.GetCell` _output_get_3 _index_6 _index_5))
                  (`MoxTDAudioInterfaceBPLibrary.HandleAbletonJsonCommands` _returnvalue_8)))
              (else
                (`KismetSystemLibrary.PrintString` "No Ableton Output :(" true true (struct :`R` 1.0 :`B` 0.06591 :`A` 1.0)))))
          (:`then_1`
            (bind (_value_6 _result_7) (`|TouchOutputK2Node` (`self.TouchEngineComponent`) "moxf_out_lisa"))
            (if _result_7
              (bind _output_get_4 (set `self.DatLisa` _value_6))
              (for _index_7 (range (- (`TouchEngineDAT.numRows` _output_get_4) 1) 1)
                (for _index_8 (range (`TouchEngineDAT.numColumns` _output_get_4))
                  (bind _returnvalue_9 (`TouchEngineDAT.GetCell` _output_get_4 _index_8 _index_7))
                  (`MoxTDAudioInterfaceBPLibrary.HandleLisaJsonCommands` _returnvalue_9)))
              (else
                (`KismetSystemLibrary.PrintString` "No Lisa Output :(" true true (struct :`R` 1.0 :`B` 0.06591 :`A` 1.0))))))))))

(event `self.ReceiveBeginPlay`
  ; ndisplay setup
  (`|ExecutionSequence`
    (:`then_0`
      (`KismetSystemLibrary.PrintString` "startup" true true (struct :`G` 0.66 :`B` 1.0 :`A` 1.0) 3.0))
    (:`then_1`
      (`DisplayClusterBlueprintLib.AddClusterEventListener` self))
    (:`then_2`
      (bind _returnvalue (`KismetSystemLibrary.GetCommandLine`))
      (bind (_outtokens _outswitches _outparams) (`KismetSystemLibrary.ParseCommandLine` _returnvalue))
      (bind (_keypin _valuepin) (`|MapForEach` _outparams)
        (:`then`
          ; error output from TD
          (`KismetSystemLibrary.PrintString` (`KismetStringLibrary.Concat_StrStr` _keypin "===>>" _valuepin)))))
    (:`then_3`
      (bind _returnvalue_2 (`|CreateWidget` "/Game/BP_NodeRenderWidget.BP_NodeRenderWidget_C" (`GameplayStatics.GetPlayerController` 0)))
      (bind _output_get (set `self.RenderWidget` _returnvalue_2))
      (`UserWidget.AddToViewport` _output_get 0))
    (:`then_4`
      (`self.StartPharusTracking`)
      (`MoxTDAudioInterfaceBPLibrary.Init` (`GameplayStatics.GetGameInstance`)))))

(event `self.TouchEngineComponent.OnToxLoaded`
  (bind _touchenginecomponent (`self.TouchEngineComponent`))
  ; TOX load events
  (`|ExecutionSequence`
    (:`then_0`
      ; LOAD signal to TD
      (`KismetSystemLibrary.Delay` 5.0)
      (bind _returnvalue (`self.GetScreenNames`))
      (bind _array (`|MakeArray` (`KismetStringLibrary.Concat_StrStr` "LOADED" ";" (`KismetStringLibrary.JoinStringArray` _returnvalue ", ") ";") "" ""))
      (bind _result (`|TouchInputK2Node` _touchenginecomponent "moxf_in_signals" _array :!label _label_3))
      (`|ExecutionSequence`
        (:`then_0`
          (`KismetSystemLibrary.PrintString` (`KismetStringLibrary.Concat_StrStr` "signal send resul:: " (`|GetArrayItem` _array) "--> " (`KismetStringLibrary.Conv_BoolToString` _result) "; PATH: " (`KismetSystemLibrary.GetPathName` _touchenginecomponent)) true true (struct :`R` 1.0 :`G` 0.223518 :`A` 1.0) 12.0))
        (:`then_1`
          (if _result
            (set `self.ToxLoaded` true)))))
    (:`then_1`
      (set `/Game/BP_NodeRenderWidget.DbgInfoPublic` (`self.toxPath`) (`self.RenderWidget`)))
    (:`then_2`
      (`KismetSystemLibrary.PrintString` "TOX LOADED." true true (struct :`G` 0.66 :`B` 1.0 :`A` 1.0) 5.0))))

(event `Key|K`
  (params (Key :type "Key Structure"))
  ; LOAD signal to TD
  (:`Released`
    (`KismetSystemLibrary.PrintString` "CCC")
    (goto _label_3)))

(event `self.TouchEngineComponent.OnToxFailedLoad`
  (params (ErrorMessage :type String))
  ; TOX load events
  (`KismetSystemLibrary.PrintString` ErrorMessage true true (struct :`R` 1.0 :`B` 0.077289 :`A` 1.0) 5.0))

(event `self.OnClusterEventBinary`
  (params (Event :type "DisplayClusterClusterEventBinary Structure (by ref)"))
  ; >> cluster node in
  (goto _label_2))

(event `Key|F12`
  (params (Key :type "Key Structure"))
  ; TOX load events
  (:`Released`
    (`TouchEngineComponentBase.LoadTox` (`self.TouchEngineComponent`) true)))

(event `self.ReceiveTick`
  (params (DeltaSeconds :type "Float (single-precision)"))
  (switch `EDisplayClusterNodeRole` (`DisplayClusterBlueprintLib.GetClusterRole`)
    (:`None`
      _)
    (:`Primary`
      _))
  ; Input and Tracking
  (`self.TransmitInputState`)
  (`self.UpdatePharusInstances`)
  (`MoxTrackingBPLibrary.UpdateTrackingData`)
  (`self.TransmitPharusState`))

(fn `AddPharusInstances`
  (bind _returnvalue (subsystem `MoxPharusSubsystem`))
  (for _array_element (`MoxPharusSubsystem.GetAllInstanceNames` _returnvalue)
    (`MoxTrackingBPLibrary.AddPharusInstanceRef` (`MoxPharusSubsystem.GetTrackerInstance` _returnvalue _array_element))))

(fn `StartPharusTracking`
  (`MoxPharusSubsystem.StartPharusSystem` (subsystem `MoxPharusSubsystem`))
  (`MoxTrackingBPLibrary.ClearPharusInstances`)
  (`self.AddPharusInstances`))

(fn `TransmitInputState`
  (`|ExecutionSequence`
    (:`then_0`
      (`|TouchInputK2Node` (`self.TouchEngineComponent`) "moxf_in_keyboard_state" (`|MakeArray` (`MoxInputBPLibrary.GetKeyboardMessage`))))
    (:`then_1`
      (`|TouchInputK2Node` (`self.TouchEngineComponent`) "moxf_in_mouse_state" (`|MakeArray` (`MoxInputBPLibrary.GetMouseMessage`))))
    (:`then_2`
      (`|TouchInputK2Node` (`self.TouchEngineComponent`) "moxf_in_gamepad_state" (`|MakeArray` (`MoxInputBPLibrary.GetGamepadMessage`))))))

(fn `TransmitPharusState`
  (`|TouchInputK2Node` (`self.TouchEngineComponent`) "moxf_in_pharus_state" (`|MakeArray` (`MoxTrackingBPLibrary.GetPharusMessage`))))

(fn `UpdatePharusInstances`
  (if (!= (`MoxTrackingBPLibrary.GetPharusInstanceCount`) (`MoxPharusSubsystem.GetInstanceCount` (subsystem `MoxPharusSubsystem`)))
    (`MoxTrackingBPLibrary.ClearPharusInstances`)
    (`self.AddPharusInstances`)))

(fn `UserConstructionScript`
  (bind _touchenginecomponent (`self.TouchEngineComponent`))
  (`|ExecutionSequence`
    (:`then_0`
      (bind _returnvalue (`self.GetScreenProcMeshes`))
      (for (_array_element _array_index) _returnvalue
        (bind _returnvalue_2 (`PrimitiveComponent.CreateDynamicMaterialInstance` _array_element 0 "/Game/td/toeOut_stereo.toeOut_stereo" "None"))
        (`KismetArrayLibrary.Array_Set` (`self.aMIDs`) _array_index _returnvalue_2 true)))
    (:`then_1`
      (bind _returnvalue_3 (`self.GetScreenNames`))
      (set `self.aScreenNames` _returnvalue_3))
    (:`then_2`
      (bind _returnvalue_4 (`KismetSystemLibrary.GetCommandLine`))
      (bind (_outtokens _outswitches _outparams) (`KismetSystemLibrary.ParseCommandLine` _returnvalue_4))
      (bind (_keypin _valuepin) (`|MapForEach` _outparams)
        (:`then`
          (`KismetSystemLibrary.PrintString` (`KismetStringLibrary.Concat_StrStr` _keypin "===>>" _valuepin)))
        (:`CompletedPin`
          (`|ExecutionSequence`
            (:`then_0`
              (bind (_value _returnvalue_5) (`BlueprintMapLibrary.Map_Find` _outparams "toxfile"))
              (if _returnvalue_5
                (bind _output_get (set `ToxAsset.FilePath` _value (`TouchEngineComponentBase.ToxAsset` _touchenginecomponent)))
                (`TouchEngineComponentBase.LoadTox` _touchenginecomponent false)
                (set `self.toxPath` _output_get)))
            (:`then_1`
              (if (`.ReturnValue` (`BlueprintMapLibrary.Map_Find` _outparams "simOnly"))
                (set `self.ProcessClusterData` false)))))))))