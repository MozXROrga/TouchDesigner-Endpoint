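; TouchEngine bridge actor that runs a TouchDesigner TOX inside an nDisplay cluster and displays its stereo output on two planes.
; Each end frame feeds two TOX textures into a shared dynamic material and prints data and error tables.
; The primary or standalone node sends input state to TD and broadcasts encoded BSON as binary cluster events.
; Received data returns to each TOX as a string array, with a flag bypassing the cluster.
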(event `self.TouchEngineComponent.OnEndFrame`
  (params (IsSuccessful :type Boolean) (Result :type "ECookFrameResult Enum" :default "Success") (FrameData :type "TouchEngineOutputFrameData Structure (by ref)"))
  (bind _datbsonin (`self.DatBsonIn`))
  (bind _touchenginecomponent (`self.TouchEngineComponent`))
  (bind _processclusterdata (`self.ProcessClusterData`))
  (bind _dynmatmesh (`self.DynMatMesh`))
  (if true
    (`|ExecutionSequence`
      (:`then_0`
        (if true
          (`|ExecutionSequence`
            (:`then_1`
              ;[0.15 0.08118 0.03921 0.5] grab frame from TD
              (bind (_value _result) (`|TouchOutputK2Node` _touchenginecomponent "moxg_out_0"))
              (if _result
                (`/Engine/EditorBlueprintResources/StandardMacros.IsValid` _dynmatmesh
                  (:`Is Valid`
                    (`MaterialInstanceDynamic.SetTextureParameterValue` _dynmatmesh "TETexIn" _value))
                  (:`Is Not Valid`
                    (`KismetSystemLibrary.PrintString` "invalid material" true true (struct :`R` 1.0 :`B` 0.233351 :`A` 1.0) :!label _label)))
                (else
                  (`KismetSystemLibrary.PrintString` "error getting output A" true true (struct :`R` 1.0 :`G` 0.119154 :`A` 1.0)))))
            (:`then_2`
              (bind (_value_2 _result_2) (`|TouchOutputK2Node` _touchenginecomponent "moxg_out_1"))
              (if _result_2
                (`/Engine/EditorBlueprintResources/StandardMacros.IsValid` _dynmatmesh
                  (:`Is Valid`
                    (`MaterialInstanceDynamic.SetTextureParameterValue` _dynmatmesh "TETexInR" _value_2))
                  (:`Is Not Valid`
                    (goto _label)))
                (else
                  (`KismetSystemLibrary.PrintString` "error getting output A2" true true (struct :`R` 1.0 :`G` 0.119154 :`A` 1.0))))))))
      (:`then_1`
        (`|ExecutionSequence`
          (:`then_0`
            ;[0.15 0.0995 0.03464 0.5] TD to DAT
            (bind (_value_3 _result_3 _framelastupdated) (`|TouchOutputK2Node` (`self.TouchEngineComponent`) "moxf_out_encoded_bson"))
            (`|ExecutionSequence`
              (:`then_0`
                (if _result_3
                  (bind _output_get (set `self.DatBsonIn` _value_3))
                  (`|ExecutionSequence`
                    (:`then_0`
                      (for _index (range (`TouchEngineDAT.numRows` _output_get))
                        (for _index_2 (range (`TouchEngineDAT.numColumns` _output_get))
                          (bind _returnvalue (`TouchEngineDAT.GetCell` _output_get _index_2 _index))
                          (`KismetSystemLibrary.PrintString` (`KismetStringLibrary.Concat_StrStr` (`self.CellText`) _returnvalue) true true (struct :`R` 1.0 :`G` 0.27474 :`B` 0.618986 :`A` 1.0) 2.0 "bsoncell"))))
                    (:`then_1`
                      ; send to cluster nodes >>
                      (switch `EDisplayClusterNodeRole` (`DisplayClusterBlueprintLib.GetClusterRole`)
                        (:`None`
                          _)
                        (:`Primary`
                          _))
                      (`/Engine/EditorBlueprintResources/StandardMacros.IsValid` _datbsonin
                        (:`Is Valid`
                          (bind _returnvalue_2 (`TouchEngineDAT.GetCell` _datbsonin 0 0))
                          (bind _returnvalue_3 (`MoxTdUtilBPLibrary.StringToBytes` _returnvalue_2))
                          ;; cluster event / bypass switch
                          (if _processclusterdata
                            (`DisplayClusterBlueprintLib.EmitClusterEventBinary` (make `DisplayClusterClusterEventBinary` 1 _returnvalue_3))
                            (`KismetSystemLibrary.PrintString` (`KismetStringLibrary.Concat_StrStr` "EMITTING BINARY " _returnvalue_2) true true (struct :`G` 1.0 :`B` 0.229809 :`A` 1.0) 2.0 "pri_emit")
                            (else
                              ; >> cluster node in
                              (bind _returnvalue_4 (`MoxTdUtilBPLibrary.BytesToString` (select `bool` _processclusterdata :`false` _returnvalue_3 :`true` (`.EventData` (break `DisplayClusterClusterEventBinary` (stale `self.OnClusterEventBinary` Event)))) :!label _label_2))
                              (`|ExecutionSequence`
                                (:`then_0`
                                  (`|TouchInputK2Node` (`self.TouchEngineComponent`) "moxf_in_encoded_bson" (`|MakeArray` _returnvalue_4)))
                                (:`then_1`
                                  (`KismetSystemLibrary.PrintString` (`KismetStringLibrary.Concat_StrStr` "cluster IN: " _returnvalue_4) true true (struct :`G` 0.66 :`B` 1.0 :`A` 1.0) 2.0 "cluster in")))))))))
                  (else
                    (`KismetSystemLibrary.PrintString` "FAIL get DAT" true true (struct :`R` 0.557292 :`B` 0.056032 :`A` 1.0) 1.0))))
              (:`then_1`
                (`KismetSystemLibrary.PrintString` (`KismetStringLibrary.Conv_Int64ToString` _framelastupdated) true true (struct :`R` 0.143515 :`G` 0.013095 :`B` 1.0 :`A` 1.0) 2.0 "td_dat_frame"))))
          (:`then_1`
            ; error output from TD
            (bind (_value_4 _result_4 _framelastupdated_2) (`|TouchOutputK2Node` (`self.TouchEngineComponent`) "moxf_out_err"))
            (`|ExecutionSequence`
              (:`then_0`
                (if _result_4
                  (bind _output_get_2 (set `self.DatErrIn` _value_4))
                  (`|ExecutionSequence`
                    (:`then_0`
                      (for _index_3 (range (`TouchEngineDAT.numRows` _output_get_2))
                        (for _index_4 (range (`TouchEngineDAT.numColumns` _output_get_2))
                          (bind _returnvalue_5 (`TouchEngineDAT.GetCell` _output_get_2 _index_4 _index_3))
                          (`KismetSystemLibrary.PrintString` (`KismetStringLibrary.Concat_StrStr` "ERR: " _returnvalue_5) true true (struct :`R` 1.0 :`G` 0.27474 :`B` 0.618986 :`A` 1.0) 2.0 "ERR DAT")))))
                  (else
                    (`KismetSystemLibrary.PrintString` "FAIL get DAT" true true (struct :`R` 0.557292 :`B` 0.056032 :`A` 1.0) 1.0))))
              (:`then_1`
                (`KismetSystemLibrary.PrintString` (`KismetStringLibrary.Conv_Int64ToString` _framelastupdated_2) true true (struct :`R` 0.143515 :`G` 0.013095 :`B` 1.0 :`A` 1.0) 2.0 "td_dat_frame")))))))))

(event `self.ReceiveTick`
  (params (DeltaSeconds :type "Float (single-precision)"))
  (switch `EDisplayClusterNodeRole` (`DisplayClusterBlueprintLib.GetClusterRole`)
    (:`None`
      _)
    (:`Primary`
      _))
  (`self.TransmitInputState`))

(event `self.ReceiveBeginPlay`
  ; ndisplay setup
  (`|ExecutionSequence`
    (:`then_0`
      (`KismetSystemLibrary.PrintString` "startup" true true (struct :`G` 0.66 :`B` 1.0 :`A` 1.0) 3.0))
    (:`then_1`
      (`DisplayClusterBlueprintLib.AddClusterEventListener` self))))

(event `Key|K`
  (params (Key :type "Key Structure"))
  (bind _array (`|MakeArray` (`KismetStringLibrary.Concat_StrStr` "LOADED" ":" "VP_LeftFront")))
  ; LOAD signal to TD
  (:`Released`
    (`KismetSystemLibrary.PrintString` "CCC")
    (bind _result (`|TouchInputK2Node` (`self.TouchEngineComponent`) "moxf_in_signals" _array :!label _label_3))
    (`KismetSystemLibrary.PrintString` (`KismetStringLibrary.Concat_StrStr` "signal send resul:: " (`|GetArrayItem` _array) "--> " (`KismetStringLibrary.Conv_BoolToString` _result)) true true (struct :`R` 1.0 :`G` 0.223518 :`A` 1.0) 12.0)))

(event `self.TouchEngineComponent.OnToxLoaded`
  ; TOX load events
  (`KismetSystemLibrary.PrintString` "TOX LOADED." true true (struct :`G` 0.66 :`B` 1.0 :`A` 1.0) 5.0)
  (goto _label_3))

(event `self.TouchEngineComponent.OnToxFailedLoad`
  (params (ErrorMessage :type String))
  ; TOX load events
  (`KismetSystemLibrary.PrintString` ErrorMessage true true (struct :`R` 1.0 :`B` 0.077289 :`A` 1.0) 5.0))

(event `self.OnClusterEventBinary`
  (params (Event :type "DisplayClusterClusterEventBinary Structure (by ref)"))
  ; >> cluster node in
  (goto _label_2))

(event `Key|F12`
  (params (Key :type "Key Structure"))
  ; TOX load events
  (:`Released`
    (`TouchEngineComponentBase.LoadTox` (`self.TouchEngineComponent`) true)))

(fn `TransmitInputState`
  (`|ExecutionSequence`
    (:`then_0`
      (`|TouchInputK2Node` (`self.TouchEngineComponent`) "moxf_in_keyboard_state" (`|MakeArray` (`MoxInputBPLibrary.GetKeyboardMessage`))))
    (:`then_1`
      (`|TouchInputK2Node` (`self.TouchEngineComponent`) "moxf_in_mouse_state" (`|MakeArray` (`MoxInputBPLibrary.GetMouseMessage`))))
    (:`then_2`
      (`|TouchInputK2Node` (`self.TouchEngineComponent`) "moxf_in_gamepad_state" (`|MakeArray` (`MoxInputBPLibrary.GetGamepadMessage`))))))

(fn `UserConstructionScript`
  (bind _returnvalue (`self.GetParentActor`))
  (`|ExecutionSequence`
    (:`then_0`
      (bind _returnvalue_2 (`PrimitiveComponent.CreateDynamicMaterialInstance` (`self.Plane`) 0 "/Game/td/toeOut_stereo.toeOut_stereo" "None"))
      (bind _output_get (set `self.DynMatMesh` _returnvalue_2))
      (`PrimitiveComponent.SetMaterial` (`self.Plane1`) 0 _output_get))
    (:`then_1`
      (set `self.parent` _returnvalue)
      (`KismetSystemLibrary.PrintString` (`KismetSystemLibrary.GetDisplayName` _returnvalue) true true (struct :`G` 0.66 :`B` 1.0 :`A` 1.0) 2.0 "PARENT:::: "))))