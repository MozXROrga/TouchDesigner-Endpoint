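; BP_Input is an input relay that captures keyboard, mouse and gamepad state and passes it to register and setter functions.
; BeginPlay enables input from player controller 0, and Tick reports the mouse position divided by viewport size.
; Any Key events register presses and releases by display name and print that name on screen.
; Gamepad buttons, stick axes and trigger axes map to fixed integer indices.
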(event `Key|AnyKey`
  (params (Key :type "Key Structure"))
  (bind _returnvalue (`KismetTextLibrary.Conv_TextToString` (`KismetInputLibrary.Key_GetDisplayName` Key)))
  (:`Pressed`
    (`MoxInputBPLibrary.RegisterKeyPressed` _returnvalue)
    (`KismetSystemLibrary.PrintString` _returnvalue true true (struct :`G` 1.0 :`B` 0.071833 :`A` 1.0) :!label _label))
  (:`Released`
    (`MoxInputBPLibrary.RegisterKeyReleased` _returnvalue)
    (goto _label)))

(event `self.ReceiveBeginPlay`
  (`self.EnableInput` (`GameplayStatics.GetPlayerController` 0)))

(event `self.ReceiveTick`
  (params (DeltaSeconds :type "Float (single-precision)"))
  (bind _returnvalue (`WidgetLayoutLibrary.GetMousePositionOnViewport`))
  (bind (_x _y) (`KismetMathLibrary.BreakVector2D` (/ _returnvalue (`WidgetLayoutLibrary.GetViewportSize`))))
  (`MoxInputBPLibrary.SetMousePosition` _x _y))

(event `Key|Gamepad_FaceButton_Top`
  (params (Key :type "Key Structure"))
  (:`Pressed`
    (`MoxInputBPLibrary.RegisterGamepadPressed` 3))
  (:`Released`
    (`MoxInputBPLibrary.RegisterGamepadReleased` 3)))

(event `Key|Gamepad_DPad_Down`
  (params (Key :type "Key Structure"))
  (:`Pressed`
    (`MoxInputBPLibrary.RegisterGamepadPressed` 10))
  (:`Released`
    (`MoxInputBPLibrary.RegisterGamepadReleased` 10)))

(event `InputAxisKey|Gamepad_LeftX`
  (params (AxisValue :type "Float (single-precision)"))
  (`MoxInputBPLibrary.SetGamepadAxisValue` 0 AxisValue))

(event `InputAxisKey|Gamepad_LeftY`
  (params (AxisValue :type "Float (single-precision)"))
  (`MoxInputBPLibrary.SetGamepadAxisValue` 1 AxisValue))

(event `Key|Gamepad_FaceButton_Bottom`
  (params (Key :type "Key Structure"))
  (:`Pressed`
    (`MoxInputBPLibrary.RegisterGamepadPressed` 0))
  (:`Released`
    (`MoxInputBPLibrary.RegisterGamepadReleased` 0)))

(event `Key|Gamepad_DPad_Right`
  (params (Key :type "Key Structure"))
  (:`Pressed`
    (`MoxInputBPLibrary.RegisterGamepadPressed` 11))
  (:`Released`
    (`MoxInputBPLibrary.RegisterGamepadReleased` 11)))

(event `InputAxisKey|Gamepad_RightX`
  (params (AxisValue :type "Float (single-precision)"))
  (`MoxInputBPLibrary.SetGamepadAxisValue` 2 AxisValue))

(event `Key|Gamepad_FaceButton_Left`
  (params (Key :type "Key Structure"))
  (:`Pressed`
    (`MoxInputBPLibrary.RegisterGamepadPressed` 2))
  (:`Released`
    (`MoxInputBPLibrary.RegisterGamepadReleased` 2)))

(event `Key|Gamepad_DPad_Left`
  (params (Key :type "Key Structure"))
  (:`Pressed`
    (`MoxInputBPLibrary.RegisterGamepadPressed` 12))
  (:`Released`
    (`MoxInputBPLibrary.RegisterGamepadReleased` 12)))

(event `InputAxisKey|Gamepad_RightY`
  (params (AxisValue :type "Float (single-precision)"))
  (`MoxInputBPLibrary.SetGamepadAxisValue` 3 AxisValue))

(event `InputAxisKey|Gamepad_LeftTriggerAxis`
  (params (AxisValue :type "Float (single-precision)"))
  (`MoxInputBPLibrary.SetGamepadAxisValue` 4 AxisValue))

(event `Key|Gamepad_FaceButton_Right`
  (params (Key :type "Key Structure"))
  (:`Pressed`
    (`MoxInputBPLibrary.RegisterGamepadPressed` 1))
  (:`Released`
    (`MoxInputBPLibrary.RegisterGamepadReleased` 1)))

(event `Key|Gamepad_DPad_Up`
  (params (Key :type "Key Structure"))
  (:`Pressed`
    (`MoxInputBPLibrary.RegisterGamepadPressed` 13))
  (:`Released`
    (`MoxInputBPLibrary.RegisterGamepadReleased` 13)))

(event `InputAxisKey|Gamepad_RightTriggerAxis`
  (params (AxisValue :type "Float (single-precision)"))
  (`MoxInputBPLibrary.SetGamepadAxisValue` 5 AxisValue))

(event `Key|Gamepad_LeftShoulder`
  (params (Key :type "Key Structure"))
  (:`Pressed`
    (`MoxInputBPLibrary.RegisterGamepadPressed` 4))
  (:`Released`
    (`MoxInputBPLibrary.RegisterGamepadReleased` 4)))

(event `Key|Gamepad_RightShoulder`
  (params (Key :type "Key Structure"))
  (:`Pressed`
    (`MoxInputBPLibrary.RegisterGamepadPressed` 5))
  (:`Released`
    (`MoxInputBPLibrary.RegisterGamepadReleased` 5)))

(event `Key|Gamepad_Special_Left`
  (params (Key :type "Key Structure"))
  (:`Pressed`
    (`MoxInputBPLibrary.RegisterGamepadPressed` 6))
  (:`Released`
    (`MoxInputBPLibrary.RegisterGamepadReleased` 6)))

(event `Key|Gamepad_Special_Right`
  (params (Key :type "Key Structure"))
  (:`Pressed`
    (`MoxInputBPLibrary.RegisterGamepadPressed` 7))
  (:`Released`
    (`MoxInputBPLibrary.RegisterGamepadReleased` 7)))

(event `Key|Gamepad_LeftThumbstick`
  (params (Key :type "Key Structure"))
  (:`Pressed`
    (`MoxInputBPLibrary.RegisterGamepadPressed` 8))
  (:`Released`
    (`MoxInputBPLibrary.RegisterGamepadReleased` 8)))

(event `Key|Gamepad_RightThumbstick`
  (params (Key :type "Key Structure"))
  (:`Pressed`
    (`MoxInputBPLibrary.RegisterGamepadPressed` 9))
  (:`Released`
    (`MoxInputBPLibrary.RegisterGamepadReleased` 9)))

(fn `UserConstructionScript`)