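; nDisplay actor that hosts a TouchEngine TOX and shows its per-screen stereo output on a screen mesh via a dynamic material.
; After load it sends TouchDesigner the screen name and config filename, then pulls textures each engine frame.
; The primary or standalone instance relays TouchDesigner's encoded BSON as binary cluster events, which listeners feed back into TouchDesigner, with a local bypass switch.
; Debug prints and reload/resend keys aid testing.
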(event `self.TouchEngineComponent.OnEndFrame`
  (params (IsSuccessful :type Boolean) (Result :type "ECookFrameResult Enum" :default "Success") (FrameData :type "TouchEngineOutputFrameData Structure (by ref)"))
  (bind _datbsonin (`self.DatBsonIn`))
  (bind _mid_mesh (`self.MID_Mesh`))
  (bind _touchenginecomponent (`self.TouchEngineComponent`))
  (bind _processclusterdata (`self.ProcessClusterData`))
  (if (`self.ToxLoaded`)
    (`|ExecutionSequence`
      (:`then_0`
        (if true
          (`|ExecutionSequence`
            (:`then_0`
              ;[0.15 0.08118 0.03921 0.5] grab frame from TD
              (bind _returnvalue (`self.GetScreenName`)))
            (:`then_1`
              (bind _returnvalue_2 (`KismetStringLibrary.Concat_StrStr` "moxg_out_" _returnvalue))
              (bind (_value _result) (`|TouchOutputK2Node` _touchenginecomponent (`KismetStringLibrary.Concat_StrStr` _returnvalue_2 "_r")))
              (if _result
                (`/Engine/EditorBlueprintResources/StandardMacros.IsValid` _mid_mesh
                  (:`Is Valid`
                    (`MaterialInstanceDynamic.SetTextureParameterValue` _mid_mesh "TETexIn" _value))
                  (:`Is Not Valid`
                    (`KismetSystemLibrary.PrintString` "invalid material" true true (struct :`R` 1.0 :`B` 0.233351 :`A` 1.0) :!label _label)))
                (else
                  (`KismetSystemLibrary.PrintString` "error getting output R" true true (struct :`R` 1.0 :`G` 0.119154 :`A` 1.0)))))
            (:`then_2`
              (bind (_value_2 _result_2) (`|TouchOutputK2Node` _touchenginecomponent (`KismetStringLibrary.Concat_StrStr` _returnvalue_2 "_l")))
              (if _result_2
                (`/Engine/EditorBlueprintResources/StandardMacros.IsValid` _mid_mesh
                  (:`Is Valid`
                    (`MaterialInstanceDynamic.SetTextureParameterValue` _mid_mesh "TETexInR" _value_2))
                  (:`Is Not Valid`
                    (goto _label)))
                (else
                  (`KismetSystemLibrary.PrintString` "error getting output L" true true (struct :`R` 1.0 :`G` 0.119154 :`A` 1.0))))))))
      (:`then_1`
        (`|ExecutionSequence`
          (:`then_0`
            ;[0.15 0.0995 0.03464 0.5] TD to DAT
            (bind (_value_3 _result_3 _framelastupdated) (`|TouchOutputK2Node` (`self.TouchEngineComponent`) "moxf_out_encoded_bson"))
            (`|ExecutionSequence`
              (:`then_0`
                (if _result_3
                  (bind _output_get (set `self.DatBsonIn` _value_3))
                  (`|ExecutionSequence`
                    (:`then_0`
                      (for _index (range (`TouchEngineDAT.numRows` _output_get))
                        (for _index_2 (range (`TouchEngineDAT.numColumns` _output_get))
                          (bind _returnvalue_3 (`TouchEngineDAT.GetCell` _output_get _index_2 _index))
                          (`KismetSystemLibrary.PrintString` (`KismetStringLibrary.Concat_StrStr` (`self.CellText`) _returnvalue_3) true true (struct :`R` 1.0 :`G` 0.27474 :`B` 0.618986 :`A` 1.0) 2.0 "bsoncell"))))
                    (:`then_1`
                      ; send to cluster nodes >>
                      (switch `EDisplayClusterNodeRole` (`DisplayClusterBlueprintLib.GetClusterRole`)
                        (:`None`
                          _)
                        (:`Primary`
                          _))
                      (`/Engine/EditorBlueprintResources/StandardMacros.IsValid` _datbsonin
                        (:`Is Valid`
                          (bind _returnvalue_4 (`TouchEngineDAT.GetCell` _datbsonin 0 0))
                          (bind _returnvalue_5 (`MoxTdUtilBPLibrary.StringToBytes` _returnvalue_4))
                          ;; cluster event / bypass switch
                          (if _processclusterdata
                            (`DisplayClusterBlueprintLib.EmitClusterEventBinary` (make `DisplayClusterClusterEventBinary` 1 _returnvalue_5))
                            (`KismetSystemLibrary.PrintString` (`KismetStringLibrary.Concat_StrStr` "EMITTING BINARY " _returnvalue_4) true true (struct :`G` 1.0 :`B` 0.229809 :`A` 1.0) 2.0 "pri_emit")
                            (else
                              ; >> cluster node in
                              (bind _returnvalue_6 (`MoxTdUtilBPLibrary.BytesToString` (select `bool` _processclusterdata :`false` _returnvalue_5 :`true` (`.EventData` (break `DisplayClusterClusterEventBinary` (stale `self.OnClusterEventBinary` Event)))) :!label _label_2))
                              (`|ExecutionSequence`
                                (:`then_0`
                                  (`|TouchInputK2Node` (`self.TouchEngineComponent`) "moxf_in_encoded_bson" (`|MakeArray` _returnvalue_6)))
                                (:`then_1`
                                  (`KismetSystemLibrary.PrintString` (`KismetStringLibrary.Concat_StrStr` "cluster IN: " _returnvalue_6) true true (struct :`G` 0.66 :`B` 1.0 :`A` 1.0) 2.0 "cluster in")))))))))
                  (else
                    (`KismetSystemLibrary.PrintString` "FAIL get DAT" true true (struct :`R` 0.557292 :`B` 0.056032 :`A` 1.0) 1.0))))
              (:`then_1`
                (`KismetSystemLibrary.PrintString` (`KismetStringLibrary.Conv_Int64ToString` _framelastupdated) true true (struct :`R` 0.143515 :`G` 0.013095 :`B` 1.0 :`A` 1.0) 2.0 "td_dat_frame"))))
          (:`then_1`
            ; error output from TD
            (bind (_value_4 _result_4 _framelastupdated_2) (`|TouchOutputK2Node` (`self.TouchEngineComponent`) "moxf_out_err"))
            (`|ExecutionSequence`
              (:`then_0`
                (if _result_4
                  (bind _output_get_2 (set `self.DatErrIn` _value_4))
                  (`|ExecutionSequence`
                    (:`then_0`
                      (for _index_3 (range (`TouchEngineDAT.numRows` _output_get_2))
                        (for _index_4 (range (`TouchEngineDAT.numColumns` _output_get_2))
                          (bind _returnvalue_7 (`TouchEngineDAT.GetCell` _output_get_2 _index_4 _index_3))
                          (`KismetSystemLibrary.PrintString` (`KismetStringLibrary.Concat_StrStr` "ERR: " _returnvalue_7) true true (struct :`R` 1.0 :`G` 0.27474 :`B` 0.618986 :`A` 1.0) 2.0 "ERR DAT")))))
                  (else
                    (`KismetSystemLibrary.PrintString` "FAIL get DAT" true true (struct :`R` 0.557292 :`B` 0.056032 :`A` 1.0) 1.0))))
              (:`then_1`
                (`KismetSystemLibrary.PrintString` (`KismetStringLibrary.Conv_Int64ToString` _framelastupdated_2) true true (struct :`R` 0.143515 :`G` 0.013095 :`B` 1.0 :`A` 1.0) 2.0 "td_dat_frame")))))))))

(event `self.ReceiveBeginPlay`
  ; ndisplay setup
  (`|ExecutionSequence`
    (:`then_0`
      (`KismetSystemLibrary.PrintString` "startup" true true (struct :`G` 0.66 :`B` 1.0 :`A` 1.0) 3.0))
    (:`then_1`
      (`DisplayClusterBlueprintLib.AddClusterEventListener` self))
    (:`then_2`
      (bind _returnvalue (`KismetSystemLibrary.GetCommandLine`))
      (bind (_outtokens _outswitches _outparams) (`KismetSystemLibrary.ParseCommandLine` _returnvalue))
      (bind (_keypin _valuepin) (`|MapForEach` _outparams)
        (:`then`
          ; error output from TD
          (`KismetSystemLibrary.PrintString` (`KismetStringLibrary.Concat_StrStr` _keypin "===>>" _valuepin)))))))

(event `Key|K`
  (params (Key :type "Key Structure"))
  (bind _touchenginecomponent (`self.TouchEngineComponent`))
  ; LOAD signal to TD
  (:`Released`
    (`KismetSystemLibrary.PrintString` "CCC")
    (bind _array (`|MakeArray` (`KismetStringLibrary.Concat_StrStr` "LOADED" ";" (stale `self.TouchEngineComponent.OnToxLoaded` _returnvalue_2) ";" (stale `self.TouchEngineComponent.OnToxLoaded` _returnvalue)) "" ""))
    (bind _result (`|TouchInputK2Node` _touchenginecomponent "moxf_in_signals" _array :!label _label_3))
    (`|ExecutionSequence`
      (:`then_0`
        (`KismetSystemLibrary.PrintString` (`KismetStringLibrary.Concat_StrStr` "signal send resul:: " (`|GetArrayItem` _array) "--> " (`KismetStringLibrary.Conv_BoolToString` _result) "; PATH: " (`KismetSystemLibrary.GetPathName` _touchenginecomponent)) true true (struct :`R` 1.0 :`G` 0.223518 :`A` 1.0) 12.0))
      (:`then_1`
        (if _result
          (set `self.ToxLoaded` true))))))

(event `self.TouchEngineComponent.OnToxLoaded`
  ; TOX load events
  (`|ExecutionSequence`
    (:`then_1`
      ; LOAD signal to TD
      (`KismetSystemLibrary.Delay` 5.0)
      (bind _returnvalue (`self.GetConfigFilename`))
      (bind _returnvalue_2 (`self.GetScreenName`))
      (goto _label_3))
    (:`then_2`
      (`KismetSystemLibrary.PrintString` "TOX LOADED." true true (struct :`G` 0.66 :`B` 1.0 :`A` 1.0) 5.0))))

(event `self.TouchEngineComponent.OnToxFailedLoad`
  (params (ErrorMessage :type String))
  ; TOX load events
  (`KismetSystemLibrary.PrintString` ErrorMessage true true (struct :`R` 1.0 :`B` 0.077289 :`A` 1.0) 5.0))

(event `self.OnClusterEventBinary`
  (params (Event :type "DisplayClusterClusterEventBinary Structure (by ref)"))
  ; >> cluster node in
  (goto _label_2))

(event `Key|F12`
  (params (Key :type "Key Structure"))
  ; TOX load events
  (:`Released`
    (`TouchEngineComponentBase.LoadTox` (`self.TouchEngineComponent`) true)))

(fn `UserConstructionScript`
  (`|ExecutionSequence`
    (:`then_0`
      (bind _returnvalue (`MoxClusterSimulatorCustomActor.GetScreenProcMesh`))
      (bind _returnvalue_2 (`PrimitiveComponent.CreateDynamicMaterialInstance` _returnvalue 0 "/Game/td/toeOut_stereo.toeOut_stereo" "None"))
      (set `self.MID_Mesh` _returnvalue_2))))